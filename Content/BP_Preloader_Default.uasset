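; Default preloader Blueprint that warms up materials, static meshes and Niagara systems by spawning a temporary loader actor for each asset.
; Each PreLoad function spawns its matching loader (Mat, Mesh or Niagara) at a default transform with the asset passed in, caches it and returns it.
; OnLoadFinish destroys all cached loaders and clears the list, while PostLoadedCount is left empty.
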(event EventBeginPlay)

(event Collision|EventActorBeginOverlap
  (params (OtherActor :type Actor%20Object%20Reference)))

(event EventTick
  (params (DeltaSeconds :type Float%20%28single-precision%29)))

(event EventPostLoadedCount
  (params (LoadedCount :type Integer)))

(event EventOnLoadFinish
  (for _array_element (Variables|Default|GetCachedLoader)
    (Actor|DestroyActor _array_element))
  (Utilities|Array|Clear (Variables|Default|GetCachedLoader)))

(fn ConstructionScript)

(fn PreLoadMaterial
  (params (Material :type Material%20Soft%20Object%20Reference%20%28by%20ref%29))
  (bind _returnvalue (Game|SpawnActorfromClass "/LomoLib/BP_Mat_Loader.BP_Mat_Loader_C" (Variables|Default|GetDefaultLoaderTransform) "Undefined" "MultiplyWithRoot" 0 Material 0))
  (Utilities|Array|Add (Variables|Default|GetCachedLoader) _returnvalue)
  (return _returnvalue))

(fn PreLoadStaticMesh
  (params (StaticMesh :type Static%20Mesh%20Soft%20Object%20Reference%20%28by%20ref%29))
  (bind _returnvalue (Game|SpawnActorfromClass "/LomoLib/BP_Mesh_Loader.BP_Mesh_Loader_C" (Variables|Default|GetDefaultLoaderTransform) "Undefined" "MultiplyWithRoot" 0 StaticMesh 0))
  (Utilities|Array|Add (Variables|Default|GetCachedLoader) _returnvalue)
  (return _returnvalue))

(fn PreLoadNiagaraSystem
  (params (NiagaraSystem :type Niagara%20System%20Soft%20Object%20Reference%20%28by%20ref%29))
  (bind _returnvalue (Game|SpawnActorfromClass "/LomoLib/BP_Niagara_Loader.BP_Niagara_Loader_C" (Variables|Default|GetDefaultLoaderTransform) "Undefined" "MultiplyWithRoot" 0 NiagaraSystem 0))
  (Utilities|Array|Add (Variables|Default|GetCachedLoader) _returnvalue)
  (return _returnvalue))